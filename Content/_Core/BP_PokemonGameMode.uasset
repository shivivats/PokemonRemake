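; Game mode for turn-based Pokémon battles that resolves player and opponent attacks.
; Player attacks require the GameState's PlayerTurn flag, opponent attacks skip that check, and both then call OnTurnEnd.
; Shared PokemonAttack checks PP, then damages the defender by attack/defense ratio times base power with 0.9–1.0 variance, using GameState stats.
; PP decrement and battle message nodes are disconnected, so PP never drops here.
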(fn ConstructionScript)

(fn PlayerPokemonAttack
  (params (AttackStruct :type F%20Pokemon%20Attack%20Structure%20%28by%20ref%29))
  (bind _asbp_pokemon_game_state (Utilities|Casting|CastToBP_PokemonGameState (Game|GetGameState)))
  (if (Variables|/Game/_Core/BP_PokemonGameState.BP_PokemonGameState_C|GetPlayerTurn _asbp_pokemon_game_state)
    (CallFunction|PokemonAttack AttackStruct)
    ;[1 1 1] Call OnTurnEnd with PlayerTurnEnded true
    (CallFunction|OnTurnEnd true)
    (Development|PrintString "player turn ended" true true "(R=1.000000,G=0.000000,B=0.533333,A=1.000000)")))

(fn OpponentPokemonAttack
  (params (Attack :type F%20Pokemon%20Attack%20Structure))
  (CallFunction|PokemonAttack Attack)
  ;[1 1 1] Call OnTurnEnd with PlayerTurnEnded false
  (CallFunction|OnTurnEnd false)
  (Development|PrintString "Opponent Turn ended" true true "(R=1.000000,G=0.000000,B=0.533333,A=1.000000)"))

(fn PokemonAttack
  (params (Attack :type F%20Pokemon%20Attack%20Structure%20%28by%20ref%29))
  ;[1 1 1] Check if enough pp for the attack
  (if (> (Utilities|Struct|BreakFPokemonAttack Attack) 0)
    ;[1 1 1] Get attack and defense and do damage to appropriate Pokemon's health
    (bind _asbp_pokemon_game_state (Utilities|Casting|CastToBP_PokemonGameState (Game|GetGameState)))
    (bind (_attackerattack _defenderdefense) (Default|GetAttackStats _asbp_pokemon_game_state))
    (bind (_attacker _defender) (Default|GetBattlePokemons _asbp_pokemon_game_state))
    (Default|ChangeHealth (Variables|/Game/Pokemon/_Blueprints/BP_PokemonBase.BP_PokemonBase_C|GetPokemonAttributeComponent _defender) (* (Math|Float|Round (* (* (/ _attackerattack _defenderdefense) (.BasePower (Utilities|Struct|BreakFPokemonAttack Attack))) (Math|Random|RandomFloatinRange 0.9 1.0))) -1))))