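; Player character for a Pokémon game that starts a battle when it overlaps a Pokémon and handles the switch in and out of battle.
; Overlap calls BP_BattleManager, whose begin and end events toggle input mode and third-person versus first-person cameras.
; Battle start also repositions the player, halts the opponent's AI, spawns the first collection Pokémon and passes it to the game mode.
; A delay after battle end prevents immediate re-triggering.
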(event Custom|OnBattleStart
  (bind _returnvalue (Transformation|GetActorForwardVector))
  (bind _returnvalue_2 (Transformation|GetActorLocation))
  (bind _returnvalue_3 (* _returnvalue (Math|Vector|MakeVector 1e+02 1e+02 1e+02)))
  (bind _returnvalue_4 (+ _returnvalue_2 _returnvalue_3))
  (Variables|Default|SetInBattle true)
  ;[1 1 1] Set player controller to UI only
  (bind _asbp_pokemon_player_controller (Utilities|Casting|CastToBP_PokemonPlayerController (Pawn|GetController)))
  (Input|SetInputModeUIOnly _asbp_pokemon_player_controller 0 "DoNotLock" true)
  (Variables|/Script/Engine.MovementComponent|SetVelocity (Variables|Character|GetCharacterMovement) "0, 0, 0")
  ;[1 1 1] Change player camera to first person
  (Components|Activation|Deactivate (Variables|Default|GetFollowCamera))
  (Components|Activation|Activate (Variables|Default|GetFirstPersonBattleCamera) false)
  (Variables|Default|SetbUseControllerRotationYaw true) ; Do this for first person so we can look independent of the camera
  ;[1 1 1] Set player location away from opponent Pokemon - in the future we can set both the Pokemon and the player to be offset some amount from the middle point
  (Transformation|SetActorLocationAndRotation (+ (Transformation|GetActorLocation) (* (Transformation|GetActorForwardVector) (Math|Vector|MakeVector -5e+02 -5e+02 -5e+02))) "0, 0, 0" true true)
  ;[1 1 1] Set opponent Pokemon's rotation to look at character
  (Transformation|SetActorRotation 0 (Math|Rotator|FindLookatRotation (Transformation|GetActorLocation) (Transformation|GetActorLocation)))
  ;[1 1 1] Disable movement of opponent Pokemon AI
  (bind _asaic_pokemon (Utilities|Casting|CastToAIC_Pokemon (AI|GetAIController 0)))
  (AI|Navigation|StopMovement _asaic_pokemon)
  (AI|Components|Blackboard|SetValueasBool (AI|GetBlackboard _asaic_pokemon) (Utilities|Name|MakeLiteralName "CanMove") false)
  ;[1 1 1] Spawn new Pokemon
  (bind _returnvalue_5 (Game|SpawnActorfromClass (Utilities|Array|Get(acopy) (Variables|/Game/_Core/BP_PokemonCollectionComponent.BP_PokemonCollectionComponent_C|GetPokemons (Variables|Default|GetPokemonCollectionComponent))) (Math|Transform|MakeTransform _returnvalue_4 (Math|Rotator|FindLookatRotation _returnvalue_4 (Transformation|GetActorLocation)) "1.000000,1.000000,1.000000") "AdjustIfPossibleButAlwaysSpawn" "MultiplyWithRoot" 0 self))
  ;[1 1 1] Set UI according to player Pokemon's attacks
  (bind _output_get (Variables|Default|SetSpawnedPokemon _returnvalue_5))
  (bind _asbp_pokemon_game_mode (Utilities|Casting|CastToBP_PokemonGameMode (Game|GetGameMode)))
  (Default|OnBattleBegin _asbp_pokemon_game_mode _output_get 0))

(event Custom|BattleEnded
  ;[1 1 1] Set player character back to normal controls
  (bind _asbp_pokemon_player_controller (Utilities|Casting|CastToBP_PokemonPlayerController (Pawn|GetController)))
  (Input|SetInputModeGameOnly _asbp_pokemon_player_controller false)
  ;[1 1 1] Set camera back to third-person
  (Components|Activation|Deactivate (Variables|Default|GetFirstPersonBattleCamera))
  (Components|Activation|Activate (Variables|Default|GetFollowCamera) false)
  (Variables|Default|SetbUseControllerRotationYaw false)
  ;[1 1 1] Set InBattle to false after a delay to prevent another battle starting quickly after exiting this one
  (Utilities|FlowControl|Delay 5.0)
  (Variables|Default|SetInBattle false))

(event EventBeginPlay
  (bind _returnvalue (Actor|GetActorOfClass "/Game/_Core/Battle/BP_BattleManager.BP_BattleManager_C"))
  (EventDispatchers|BindEventtoOnBattleEnd _returnvalue (delegate Custom|BattleEnded))
  (EventDispatchers|BindEventtoOnBattleBegin _returnvalue (delegate Custom|OnBattleStart)))

(event Collision|EventActorBeginOverlap
  (params (OtherActor :type Actor%20Object%20Reference))
  (if (not (Variables|Default|GetInBattle))
    (bind _asbp_pokemon_base (Utilities|Casting|CastToBP_PokemonBase OtherActor)) ; Upon collision with a pokemon, we want to do a few things:\n1. change player control to UI only\n2. chagne the camera to first person or to a special battle cam\n3. disable movement of other pokemon\n4. spawn the first pokemon from the pokemon collecton component\n5. make battle hud based on the spawned pokemon's attacks
    (bind _returnvalue (Actor|GetActorOfClass "/Game/_Core/Battle/BP_BattleManager.BP_BattleManager_C"))
    (Default|BeginBattle _returnvalue 0 _asbp_pokemon_base)
    (Development|PrintString "Overlapping with other actor")))

(fn ConstructionScript)