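; Game state for a turn-based Pokemon battle that resolves which side is attacking and which is defending.
; Both functions branch on PlayerTurn to assign the player's and opponent's Pokemon to the attacker and defender roles.
; GetBattlePokemons returns the two Pokemon, while GetAttackStats reads the attacker's Attack and the defender's Defense from their attribute components.
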(event EventBeginPlay)

(event EventTick
  (params (DeltaSeconds :type Float%20%28single-precision%29)))

(fn ConstructionScript)

(fn GetAttackStats
  (if (Variables|Default|GetPlayerTurn)
    (return (Variables|/Game/Pokemon/_Components/BP_PokemonAttributeComponent.BP_PokemonAttributeComponent_C|GetAttack (Variables|/Game/Pokemon/_Blueprints/BP_PokemonBase.BP_PokemonBase_C|GetPokemonAttributeComponent (Variables|Default|GetPlayerPokemon))) (Variables|/Game/Pokemon/_Components/BP_PokemonAttributeComponent.BP_PokemonAttributeComponent_C|GetDefense (Variables|/Game/Pokemon/_Blueprints/BP_PokemonBase.BP_PokemonBase_C|GetPokemonAttributeComponent (Variables|Default|GetOpponentPokemon))))
    (else
      (return (Variables|/Game/Pokemon/_Components/BP_PokemonAttributeComponent.BP_PokemonAttributeComponent_C|GetAttack (Variables|/Game/Pokemon/_Blueprints/BP_PokemonBase.BP_PokemonBase_C|GetPokemonAttributeComponent (Variables|Default|GetOpponentPokemon))) (Variables|/Game/Pokemon/_Components/BP_PokemonAttributeComponent.BP_PokemonAttributeComponent_C|GetDefense (Variables|/Game/Pokemon/_Blueprints/BP_PokemonBase.BP_PokemonBase_C|GetPokemonAttributeComponent (Variables|Default|GetPlayerPokemon)))))))

(fn GetBattlePokemons
  (if (Variables|Default|GetPlayerTurn)
    (return (Variables|Default|GetPlayerPokemon) (Variables|Default|GetOpponentPokemon))
    (else
      (return (Variables|Default|GetOpponentPokemon) (Variables|Default|GetPlayerPokemon)))))