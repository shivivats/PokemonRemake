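; Battle manager actor that runs turn-based Pokémon battles between the player's first Pokémon and one they collide with.
; BeginBattle spawns the player's Pokémon facing the opponent, creates the battle HUD and switches the opponent's AI state, which EndBattle reverts.
; PokemonAttack applies Pokémon-style damage with STAB, burn, crit, randomness and type effectiveness, spends PP, then calls EndTurn.
; EndTurn alternates turns, toggling HUD input and firing event dispatchers.
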(event EventBeginPlay)

(event Collision|EventActorBeginOverlap
  (params (OtherActor :type Actor%20Object%20Reference)))

(event EventTick
  (params (DeltaSeconds :type Float%20%28single-precision%29)))

(fn ConstructionScript)

(fn BeginBattle
  (params (CollidedPokemon :type BP%20Pokemon%20Base%20Object%20Reference))
  ;[1 1 1] Spawn player pokemon
  (bind _asbp_pokemon_character (Utilities|Casting|CastToBP_PokemonCharacter (Game|GetPlayerCharacter 0)))
  (bind _pokemonclass (Default|GetFirstPokemon (Variables|/Game/_Core/BP_PokemonCharacter.BP_PokemonCharacter_C|GetPokemonCollectionComponent _asbp_pokemon_character)))
  (bind _pokemonobject (CallFunction|SpawnPokemon _pokemonclass CollidedPokemon))
  ;[1 1 1] Set Pokemons
  (bind _output_get (Variables|Pokemon|SetPlayerPokemon _pokemonobject))
  (bind _output_get_2 (Variables|Pokemon|SetOpponentPokemon CollidedPokemon))
  ;[1 1 1] Create Battle HUD
  (bind _returnvalue (UserInterface|CreateWidget "/Game/UI/WBP_BattleHUD.WBP_BattleHUD_C" (Game|GetPlayerController 0) _output_get _output_get_2))
  (UserInterface|Viewport|AddtoViewport _returnvalue 0)
  (Variables|Default|SetSpawnedBattleHUD _returnvalue)
  ;[1 1 1] Set AI Pokemon to battle state
  (bind _asaic_pokemon (Utilities|Casting|CastToAIC_Pokemon (AI|GetAIController (Variables|Pokemon|GetOpponentPokemon))))
  (Default|ChangeState _asaic_pokemon "NewEnumerator1")
  ;[1 1 1] Call the event dispatcher
  (Default|CallOnBattleBegin (Variables|Pokemon|GetPlayerPokemon) (Variables|Pokemon|GetOpponentPokemon)))

(fn EndBattle
  (bind _opponentpokemon (Variables|Pokemon|GetOpponentPokemon))
  ;[1 1 1] Set AI to overworld state and let it move again (if its still valid aka alive)
  (Utilities|IsValid _opponentpokemon
    (:Is%20Valid
      (bind _asaic_pokemon (Utilities|Casting|CastToAIC_Pokemon (AI|GetAIController _opponentpokemon)))
      (Default|ChangeState _asaic_pokemon "NewEnumerator0")
      (AI|Components|Blackboard|SetValueasBool (AI|GetBlackboard _asaic_pokemon) (Utilities|Name|MakeLiteralName "CanMove") true)
      ;[1 1 1] Destroy player pokemon
      (Actor|DestroyActor (Variables|Pokemon|GetPlayerPokemon))
      ;[1 1 1] Remove HUD
      (Widget|RemovefromParent (Variables|Default|GetSpawnedBattleHUD))
      ;[1 1 1] Call dispatcher
      (Default|CallOnBattleEnd))))

(fn EndTurn
  (bind _spawnedbattlehud (Variables|Default|GetSpawnedBattleHUD))
  (bind _playerverticalbox (Variables|/Game/UI/WBP_BattleHUD.WBP_BattleHUD_C|GetPlayerVerticalBox _spawnedbattlehud))
  (switch Utilities|FlowControl|Switch|SwitchonEBattleTurn (Variables|Default|GetCurrentTurn)
    (:NewEnumerator0
      ;[1 1 1] On player turn ended, disable the hud
      (Widget|SetIsEnabled _playerverticalbox false)
      ;[1 1 1] let AI pokemon know that it can attack
      (bind _asaic_pokemon (Utilities|Casting|CastToAIC_Pokemon (AI|GetAIController (Variables|Pokemon|GetOpponentPokemon))))
      (AI|Components|Blackboard|SetValueasBool (AI|GetBlackboard _asaic_pokemon) (Utilities|Name|MakeLiteralName "CanAttack") false)
      (Default|CallOnPlayerTurnEnd)
      ;[1 1 1] set turn to opponent
      (Variables|Default|SetCurrentTurn "NewEnumerator1"))
    (:NewEnumerator1
      ;[1 1 1] enable HUD and set turn to player
      (Widget|SetIsEnabled _playerverticalbox true)
      (Default|CallOnOpponentTurnEnd)
      (Variables|Default|SetCurrentTurn "NewEnumerator0"))))

(fn PokemonAttack
  (params (Attack :type F%20Pokemon%20Attack%20Structure%20%28by%20ref%29))
  (bind (_name _currentpp _maxpp _basepower _accuracy _type) (Utilities|Struct|BreakFPokemonAttack Attack))
  ;[1 1 1] set attacker and defender
  (switch Utilities|FlowControl|Switch|SwitchonEBattleTurn (Variables|Default|GetCurrentTurn)
    (:NewEnumerator0
      (LocalVariables|SetAttacker (Variables|Pokemon|GetPlayerPokemon))
      (LocalVariables|SetDefender (Variables|Pokemon|GetOpponentPokemon)))
    (:NewEnumerator1
      (LocalVariables|SetAttacker (Variables|Pokemon|GetOpponentPokemon))
      (LocalVariables|SetDefender (Variables|Pokemon|GetPlayerPokemon))))
  ;[1 1 1] check if enough pp for the attack
  (Default|CanAttack (Variables|/Game/Pokemon/_Core/BP_PokemonBase.BP_PokemonBase_C|GetBP_PokemonAttackComponent (LocalVariables|GetAttacker)) _name)
  (bind _damage (CallFunction|CalculateDamage _basepower _type (LocalVariables|GetAttacker) (LocalVariables|GetDefender)))
  (Default|ChangeHealth (Variables|/Game/Pokemon/_Core/BP_PokemonBase.BP_PokemonBase_C|GetPokemonAttributeComponent (LocalVariables|GetDefender)) _damage)
  (Default|ReducePP (Variables|/Game/Pokemon/_Core/BP_PokemonBase.BP_PokemonBase_C|GetBP_PokemonAttackComponent (LocalVariables|GetAttacker)) Attack 1)
  (CallFunction|EndTurn)
  (return))

(fn SpawnPokemon
  (params (PokemonClass :type BP%20Pokemon%20Base%20Class%20Reference) (OpponentMon :type BP%20Pokemon%20Base%20Object%20Reference))
  (bind _asbp_pokemon_character (Utilities|Casting|CastToBP_PokemonCharacter (Game|GetPlayerCharacter 0)))
  (bind _returnvalue (Game|SpawnActorfromClass PokemonClass (Math|Transform|MakeTransform (+ (Transformation|GetActorLocation _asbp_pokemon_character) (* (Transformation|GetActorForwardVector _asbp_pokemon_character) (Math|Vector|MakeVector 1e+02 1e+02 1e+02))) (Math|Rotator|FindLookatRotation (+ (Transformation|GetActorLocation _asbp_pokemon_character) (* (Transformation|GetActorForwardVector _asbp_pokemon_character) (Math|Vector|MakeVector 1e+02 1e+02 1e+02))) (Transformation|GetActorLocation OpponentMon)) "1.000000,1.000000,1.000000") "AdjustIfPossibleButAlwaysSpawn" "MultiplyWithRoot" 0 _asbp_pokemon_character))
  (return _returnvalue))

(fn CalculateDamage
  (params (BasePower :type Integer) (AttackType :type EPokemonType%20Enum :default "NewEnumerator18") (Attacker :type BP%20Pokemon%20Base%20Object%20Reference) (Defender :type BP%20Pokemon%20Base%20Object%20Reference))
  (bind _bp_pokemonattackcomponent (Variables|/Game/Pokemon/_Core/BP_PokemonBase.BP_PokemonBase_C|GetBP_PokemonAttackComponent Defender))
  (bind _pokemondataasset (Variables|/Game/Pokemon/_Core/BP_PokemonBase.BP_PokemonBase_C|GetPokemonDataAsset Attacker))
  (bind (_type1 _type2) (Default|GetPokemonTypes _bp_pokemonattackcomponent))
  (bind _pokemondata (Variables|/Game/Pokemon/_Data/PokemonSpecies_DataAssetBase.PokemonSpecies_DataAssetBase_C|GetPokemonData _pokemondataasset))
  (bind (_datatable _rowname) (Utilities|Struct|BreakDataTableRowHandle _pokemondata))
  ;[1 1 1] do preliminary damage calc
  (LocalVariables|SetPreliminaryDamage (+ (/ (* (/ (Variables|/Game/Pokemon/_Components/BP_PokemonAttributeComponent.BP_PokemonAttributeComponent_C|GetAttack (Variables|/Game/Pokemon/_Core/BP_PokemonBase.BP_PokemonBase_C|GetPokemonAttributeComponent Attacker)) (Variables|/Game/Pokemon/_Components/BP_PokemonAttributeComponent.BP_PokemonAttributeComponent_C|GetDefense (Variables|/Game/Pokemon/_Core/BP_PokemonBase.BP_PokemonBase_C|GetPokemonAttributeComponent Defender))) (* (+ (/ (* (Variables|/Game/Pokemon/_Core/BP_PokemonBase.BP_PokemonBase_C|GetPokemonLevel Attacker) 2) 5) 2) BasePower)) 50) 2))
  ;[1 1 1] check for STAB
  (bind _returnvalue (Utilities|GetDataTableRow _datatable _rowname)
    (:then
      (if (or (Utilities|Enum|Equal(Enum) (.Type1 (Utilities|Struct|BreakFPokemonSpeciesDataTableRow _returnvalue)) AttackType) (Utilities|Enum|Equal(Enum) (.Type2 (Utilities|Struct|BreakFPokemonSpeciesDataTableRow _returnvalue)) AttackType))
        (LocalVariables|SetOtherMultiplier (* (LocalVariables|GetOtherMultiplier) 1.5)))
      ;[1 1 1] check for burnt
      (if (Utilities|Enum|Equal(Enum) (Variables|/Game/Pokemon/_Core/BP_PokemonBase.BP_PokemonBase_C|GetStatusCondition Attacker) "NewEnumerator0")
        (LocalVariables|SetOtherMultiplier (* (LocalVariables|GetOtherMultiplier) 0.5)))
      ;[1 1 1] check for crit
      (if (< (Math|Random|RandomFloat) 0.0625)
        (LocalVariables|SetOtherMultiplier (* (LocalVariables|GetOtherMultiplier) 1.5)))
      ;[1 1 1] add the randomness between 0.85 and 1
      (LocalVariables|SetOtherMultiplier (* (LocalVariables|GetOtherMultiplier) (Math|Random|RandomFloatinRange 0.85 1.0)))
      ;[1 1 1] check type effectiveness
      (bind _typeeffectivenessmodifier (CallFunction|CaculateTypeEffectiveness AttackType (Utilities|Array|MakeArray _type1 _type2)))
      (bind _output_get (LocalVariables|SetOtherMultiplier (* _typeeffectivenessmodifier (LocalVariables|GetOtherMultiplier))))
      ;[1 1 1] get final damage value
      (bind _output_get_2 (LocalVariables|SetOtherMultiplier (* _output_get (Math|Conversions|ToFloat(Integer) (LocalVariables|GetPreliminaryDamage)))))
      (return (* (Math|Float|Truncate _output_get_2) -1)))))