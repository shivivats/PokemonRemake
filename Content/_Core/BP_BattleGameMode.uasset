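; Game mode that runs turn-based Pokemon battles between a player's Pokemon and an AI-controlled opponent.
; Battle begin spawns the HUD, stores both Pokemon in BP_BattleGameState and switches the opponent's AI state; battle end reverses this.
; Attacks spend PP and deal damage from the attack/defense ratio, base power and random variance.
; OnTurnEnd alternates turns by toggling HUD buttons, the PlayerTurn flag and the AI's CanAttack blackboard key.
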(event Custom|OnBattleBegin
  (params (PlayerMon :type BP%20Pokemon%20Base%20Object%20Reference) (OpponentMon :type BP%20Pokemon%20Base%20Object%20Reference))
  ;[1 1 1] Spawn the Battle HUD
  (bind _returnvalue (UserInterface|CreateWidget "/Game/UI/WBP_BattleHUD.WBP_BattleHUD_C" 0 PlayerMon OpponentMon))
  (UserInterface|Viewport|AddtoViewport _returnvalue 0)
  ;[1 1 1] Set appropriate pokemons in GameState
  (Variables|Default|SetSpawnedBattleHUD _returnvalue)
  (bind _asbp_battle_game_state (Utilities|Casting|CastToBP_BattleGameState (Game|GetGameState)))
  (Variables|/Game/_Core/BP_BattleGameState.BP_BattleGameState_C|SetPlayerPokemon _asbp_battle_game_state PlayerMon)
  (bind _output_get (Variables|/Game/_Core/BP_BattleGameState.BP_BattleGameState_C|SetOpponentPokemon _asbp_battle_game_state OpponentMon))
  ;[1 1 1] Set AI Pokemon state to battle
  (bind _asaic_pokemon (Utilities|Casting|CastToAIC_Pokemon (AI|GetAIController _output_get)))
  (Default|ChangeState _asaic_pokemon "NewEnumerator1"))

(event Custom|OnTurnEnd
  (params (PlayerTurnEnded :type Boolean))
  (bind _spawnedbattlehud (Variables|Default|GetSpawnedBattleHUD))
  (bind _playerverticalbox (Variables|/Game/UI/WBP_BattleHUD.WBP_BattleHUD_C|GetPlayerVerticalBox _spawnedbattlehud))
  (if PlayerTurnEnded
    ;[1 1 1] disable all player buttons
    (Widget|SetIsEnabled _playerverticalbox false)
    ;[1 1 1] Set CanAttack on AI BT to true
    (bind _asbp_battle_game_state (Utilities|Casting|CastToBP_BattleGameState (Game|GetGameState)))
    (bind _defender (Default|GetBattlePokemons _asbp_battle_game_state))
    (bind _asaic_pokemon (Utilities|Casting|CastToAIC_Pokemon (AI|GetAIController _defender)))
    (AI|Components|Blackboard|SetValueasBool (AI|GetBlackboard _asaic_pokemon) (Utilities|Name|MakeLiteralName "CanAttack") true)
    ;[1 1 1] set player turn to false in game state
    (bind _asbp_battle_game_state_2 (Utilities|Casting|CastToBP_BattleGameState (Game|GetGameState)))
    (Variables|/Game/_Core/BP_BattleGameState.BP_BattleGameState_C|SetPlayerTurn _asbp_battle_game_state_2 false)
    (else
      ;[1 1 1] Let player use the buttons again
      (Widget|SetIsEnabled _playerverticalbox true)
      ;[1 1 1] set player turn to true in game state
      (bind _asbp_battle_game_state_3 (Utilities|Casting|CastToBP_BattleGameState (Game|GetGameState)))
      (Variables|/Game/_Core/BP_BattleGameState.BP_BattleGameState_C|SetPlayerTurn _asbp_battle_game_state_3 true)
      (Development|PrintString "Player turn true"))))

(event Custom|OnBattleEnd
  (bind _asbp_battle_game_state (Utilities|Casting|CastToBP_BattleGameState (Game|GetGameState)))
  (Utilities|IsValid (Variables|/Game/_Core/BP_BattleGameState.BP_BattleGameState_C|GetOpponentPokemon _asbp_battle_game_state) ; Do this check here in case we remove the pokemon in the future (by defeating or capturing it, for example)
    (:Is%20Valid
      (bind _asaic_pokemon (Utilities|Casting|CastToAIC_Pokemon (AI|GetAIController (Variables|/Game/_Core/BP_BattleGameState.BP_BattleGameState_C|GetOpponentPokemon _asbp_battle_game_state))))
      (Default|ChangeState _asaic_pokemon "NewEnumerator0")
      (AI|Components|Blackboard|SetValueasBool (AI|GetBlackboard _asaic_pokemon) (Utilities|Name|MakeLiteralName "CanMove") true)
      (Actor|DestroyActor (Variables|/Game/_Core/BP_BattleGameState.BP_BattleGameState_C|GetPlayerPokemon _asbp_battle_game_state))
      (Widget|RemovefromParent (Variables|Default|GetSpawnedBattleHUD))
      (bind _asbp_pokemon_character (Utilities|Casting|CastToBP_PokemonCharacter (Game|Player|GetPlayerPawn 0)))
      (Default|OnBattleEnd _asbp_pokemon_character))
    (:Is%20Not%20Valid
      (Development|PrintString "opontne poeon invalid" true true "(R=1.000000,G=0.000000,B=0.002751,A=1.000000)"))))

(fn ConstructionScript)

(fn PlayerPokemonAttack
  (params (AttackStruct :type F%20Pokemon%20Attack%20Structure%20%28by%20ref%29))
  (bind _asbp_battle_game_state (Utilities|Casting|CastToBP_BattleGameState (Game|GetGameState)))
  (if (Variables|/Game/_Core/BP_BattleGameState.BP_BattleGameState_C|GetPlayerTurn _asbp_battle_game_state)
    (CallFunction|PokemonAttack AttackStruct)
    ;[1 1 1] Call OnTurnEnd with PlayerTurnEnded true
    (CallFunction|OnTurnEnd true)
    (Development|PrintString "player turn ended" true true "(R=1.000000,G=0.000000,B=0.533333,A=1.000000)")))

(fn OpponentPokemonAttack
  (params (Attack :type F%20Pokemon%20Attack%20Structure))
  (CallFunction|PokemonAttack Attack)
  ;[1 1 1] Call OnTurnEnd with PlayerTurnEnded false
  (CallFunction|OnTurnEnd false)
  (Development|PrintString "Opponent Turn ended" true true "(R=1.000000,G=0.000000,B=0.533333,A=1.000000)"))

(fn PokemonAttack
  (params (Attack :type F%20Pokemon%20Attack%20Structure%20%28by%20ref%29))
  (bind (_name _maxpp _currentpp _basepower) (Utilities|Struct|BreakFPokemonAttack Attack))
  ;[1 1 1] Check if enough pp for the attack
  (if (> (Utilities|Struct|BreakFPokemonAttack Attack) 0)
    ;[1 1 1] Get attack and defense and do damage to appropriate Pokemon's health
    (bind _asbp_battle_game_state (Utilities|Casting|CastToBP_BattleGameState (Game|GetGameState)))
    (bind (_attackerattack _defenderdefense) (Default|GetAttackStats _asbp_battle_game_state))
    (bind _defender (Default|GetBattlePokemons _asbp_battle_game_state))
    (Default|ChangeHealth (Variables|/Game/Pokemon/_Blueprints/BP_PokemonBase.BP_PokemonBase_C|GetPokemonAttributeComponent _defender) (* (Math|Float|Round (* (* (/ _attackerattack _defenderdefense) _basepower) (Math|Random|RandomFloatinRange 0.9 1.0))) -1))
    ;[1 1 1] Reduce PP by 1 after attack is done
    (bind _structout (Utilities|Struct|SetmembersinFPokemonAttack Attack (- (Utilities|Struct|BreakFPokemonAttack Attack) 1)))
    (|SetBy-RefVar Attack _structout)
    (bind (_attacker _defender_2) (Default|GetBattlePokemons _asbp_battle_game_state))
    (Development|PrintText (Utilities|Text|FormatText "{attacker} used {attack} on {defender} for {damage} damage!" (Utilities|GetDisplayName _attacker) _name (Utilities|GetDisplayName _defender_2) (* (Math|Float|Round (* (* (/ _attackerattack _defenderdefense) _basepower) (Math|Random|RandomFloatinRange 0.9 1.0))) -1)) true true "(R=1.000000,G=0.000000,B=0.048397,A=1.000000)")))