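; An actor component that tracks a Pokemon's health between configurable minimum and maximum limits.
; BeginPlay starts current health at the maximum.
; The ChangeHealth event adds a signed delta, clamps the result to the limits, and prints a debug message with the owner's name, old value, new value and delta.
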(event Custom|ChangeHealth
  (params (HealthChange :type Integer))
  (Variables|Default|SetOldHealth (Variables|Default|GetCurrentHealth))
  (bind _output_get (Variables|Default|SetCurrentHealth (Math|Integer|Clamp(Integer) (+ HealthChange (Variables|Default|GetCurrentHealth)) (Variables|Default|GetMinHealth) (Variables|Default|GetMaxHealth))))
  (Development|PrintText (Utilities|Text|FormatText "Pokemon {name} health changed from {oldHealth} to {newHealth} based on input delta of {healthDelta}." (Utilities|GetObjectName (Components|GetOwner)) (Variables|Default|GetOldHealth) _output_get HealthChange)))

(event EventBeginPlay
  (Variables|Default|SetCurrentHealth (Variables|Default|GetMaxHealth)))

(event EventTick
  (params (DeltaSeconds :type Float%20%28single-precision%29)))