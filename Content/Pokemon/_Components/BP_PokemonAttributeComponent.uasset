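; Actor component that holds a Pokémon's combat attributes: health, attack, defense and speed.
; On BeginPlay it casts its owner to BP_PokemonBase and initializes each attribute from the base values in that Pokémon's data asset, starting at full health.
; ChangeHealth applies a signed delta clamped between min and max health, prints a debug message, and fires OnHealthChanged to notify listeners.
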(event EventBeginPlay
  ;[1 1 1] Set Health
  (bind _asbp_pokemon_base (Utilities|Casting|CastToBP_PokemonBase (Components|GetOwner)))
  (bind _output_get (Variables|Health|SetMaxHealth (Variables|/Game/Pokemon/_Data/Species/PokemonSpecies_DataAssetBase.PokemonSpecies_DataAssetBase_C|GetBaseHealth (Variables|/Game/Pokemon/_Blueprints/BP_PokemonBase.BP_PokemonBase_C|GetPokemonDataAsset _asbp_pokemon_base))))
  (Variables|Health|SetCurrentHealth _output_get)
  ;[1 1 1] Set other attributes
  (Variables|Attributes|SetAttack (Variables|/Game/Pokemon/_Data/Species/PokemonSpecies_DataAssetBase.PokemonSpecies_DataAssetBase_C|GetBaseAttack (Variables|/Game/Pokemon/_Blueprints/BP_PokemonBase.BP_PokemonBase_C|GetPokemonDataAsset _asbp_pokemon_base)))
  (Variables|Attributes|SetDefense (Variables|/Game/Pokemon/_Data/Species/PokemonSpecies_DataAssetBase.PokemonSpecies_DataAssetBase_C|GetBaseDefense (Variables|/Game/Pokemon/_Blueprints/BP_PokemonBase.BP_PokemonBase_C|GetPokemonDataAsset _asbp_pokemon_base)))
  (Variables|Attributes|SetSpeed (Variables|/Game/Pokemon/_Data/Species/PokemonSpecies_DataAssetBase.PokemonSpecies_DataAssetBase_C|GetBaseSpeed (Variables|/Game/Pokemon/_Blueprints/BP_PokemonBase.BP_PokemonBase_C|GetPokemonDataAsset _asbp_pokemon_base))))

(fn ChangeHealth
  (params (HealthDelta :type Integer))
  (LocalVariables|SetOldHealth (Variables|Health|GetCurrentHealth))
  (Variables|Health|SetCurrentHealth (Math|Integer|Clamp(Integer) (+ (Variables|Health|GetCurrentHealth) HealthDelta) (Variables|Health|GetMinHealth) (Variables|Health|GetMaxHealth)))
  (Development|PrintText (Utilities|Text|FormatText "Health changed for {name} from {oldHealth} to {newHealth} with a health delta of {delta}!" (Utilities|GetDisplayName (Components|GetOwner)) (LocalVariables|GetOldHealth) (Variables|Health|GetCurrentHealth) HealthDelta))
  (Default|CallOnHealthChanged HealthDelta (Variables|Health|GetCurrentHealth) (Variables|Health|GetMaxHealth)))